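; Player-flyable spaceship that drives a physics body with thrust, pitch, yaw and roll input.
; Thrust starts at half maximum; holding Supersonic eases it quickly toward a much higher target while the axis is deflected, otherwise it eases only when the axis is near zero.
; Tick overwrites linear velocity with forward thrust plus a vertical term, computed below a speed threshold as pseudo-gravity and faded out above it.
; Rotation inputs add mass-independent torque around the ship's local axes.
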(event EventBeginPlay
  (Variables|Default|SetThrust (/ (Variables|Default|GetMaxThrust) 2.0)))

(event Collision|EventActorBeginOverlap
  (params (OtherActor :type Actor%20Object%20Reference)))

(event EventTick
  (params (DeltaSeconds :type Float%20%28single-precision%29))
  (Utilities|FlowControl|Sequence
    (:then_0
      (if (< (Math|Vector|VectorLength (Variables|Default|GetForwardVelocity)) (Variables|Default|GetGravityThreshold))
        (Variables|Default|SetUpwardVelocity (* (Math|Float|Lerp 0.0 -9.8e+02 (- (Math|Vector|VectorLength (Variables|Default|GetForwardVelocity)) (Variables|Default|GetGravityThreshold))) (Math|Vector|UnrotateVector (Math|Vector|GetUpVector (Variables|Default|GetSpaceship)) (Transformation|GetWorldRotation (Variables|Default|GetSpaceship)))))
        (else
          (Variables|Default|SetUpwardVelocity (Math|Interpolation|VInterpTo (Variables|Default|GetUpwardVelocity) "0, 0, 0" (Utilities|Time|GetWorldDeltaSeconds) 2e+01)))))
    (:then_1
      (Physics|SetPhysicsLinearVelocity (Variables|Default|GetSpaceship) (+ (Variables|Default|GetForwardVelocity) (Variables|Default|GetUpwardVelocity)) false "None"))))

(event Input|ActionEvents|InputActionSupersonic
  (params (Key :type Key%20Structure :default "None"))
  (:Pressed
    (bind _output_get (Variables|Default|SetSupersonicSpeed true)))
  (:Released
    (Variables|Default|SetSupersonicSpeed false)))

(event Input|AxisEvents|InputAxisThrust
  (params (AxisValue :type Float%20%28single-precision%29))
  (Utilities|FlowControl|Sequence
    (:then_0
      (if (stale Input|ActionEvents|InputActionSupersonic _output_get)
        (if (not (Math|Float|NearlyEqual(Float) AxisValue 0.0 0.1))
          (Variables|Default|SetThrust (Math|Interpolation|FInterpTo (Variables|Default|GetThrust) (Math|Float|Lerp 0.0 (Variables|Default|GetMaxThrust) (/ (+ AxisValue 1.0) 0.1)) (Utilities|Time|GetWorldDeltaSeconds) 1.0)))
        (elif (not (not (Math|Float|NearlyEqual(Float) AxisValue 0.0 0.1)))
          (Variables|Default|SetThrust (Math|Interpolation|FInterpTo (Variables|Default|GetThrust) (Math|Float|Lerp 0.0 (Variables|Default|GetMaxThrust) (/ (+ AxisValue 1.0) 2.0)) (Utilities|Time|GetWorldDeltaSeconds) 0.2)))))
    (:then_1
      (Variables|Default|SetForwardVelocity (* (Math|Vector|GetForwardVector (Variables|Default|GetSpaceship)) (Variables|Default|GetThrust))))))

(event Input|AxisEvents|InputAxisMoveUp
  (params (AxisValue :type Float%20%28single-precision%29))
  (Class|PrimitiveComponent|AddTorqueinDegrees (Variables|Default|GetSpaceship) (* (Math|Vector|GetRightVector (Variables|Default|GetSpaceship)) (* AxisValue (Variables|Default|GetForwardTorquePower))) "None" true))

(event Input|AxisEvents|InputAxisMoveRight
  (params (AxisValue :type Float%20%28single-precision%29))
  (Class|PrimitiveComponent|AddTorqueinDegrees (Variables|Default|GetSpaceship) (* (Math|Vector|GetUpVector (Variables|Default|GetSpaceship)) (* AxisValue (Variables|Default|GetForwardTorquePower))) "None" true))

(event Input|AxisEvents|InputAxisRoll
  (params (AxisValue :type Float%20%28single-precision%29))
  (Class|PrimitiveComponent|AddTorqueinDegrees (Variables|Default|GetSpaceship) (* (Math|Vector|GetForwardVector (Variables|Default|GetSpaceship)) (* AxisValue (Variables|Default|GetForwardTorquePower))) "None" true))

(fn ConstructionScript)