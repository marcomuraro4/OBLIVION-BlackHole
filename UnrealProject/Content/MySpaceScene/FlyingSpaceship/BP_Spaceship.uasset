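; Player-controlled flying spaceship that sets its physics linear velocity each Tick from forward thrust plus a vertical term.
; Thrust input eases thrust via FInterpTo, faster while Supersonic is held; otherwise it updates only near zero input.
; Pitch, yaw and roll inputs apply torque.
; Low speed adds a gravity-like vertical velocity, and straying over 1200 units from world origin damps velocity and resets thrust.
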(event EventBeginPlay
  (Variables|Default|SetThrust (/ (Variables|Default|GetMaxThrust) 2.0)))

(event EventTick
  (params (DeltaSeconds :type Float%20%28single-precision%29))
  (bind _spaceship (Variables|Default|GetSpaceship))
  (bind _returnvalue (Transformation|GetWorldLocation _spaceship))
  (bind _returnvalue_2 (Math|Vector|VectorLength _returnvalue))
  (bind _returnvalue_3 (/ _returnvalue_2 1e+01))
  (Utilities|FlowControl|Sequence
    (:then_0
      (if (< (Math|Vector|VectorLength (Variables|Default|GetForwardVelocity)) (Variables|Default|GetGravityThreshold))
        (Variables|Default|SetUpwardVelocity (* (Math|Float|Lerp 0.0 -9.8e+02 (- (Math|Vector|VectorLength (Variables|Default|GetForwardVelocity)) (Variables|Default|GetGravityThreshold))) (Math|Vector|UnrotateVector (Math|Vector|GetUpVector (Variables|Default|GetSpaceship)) (Transformation|GetWorldRotation (Variables|Default|GetSpaceship)))))
        (else
          (Variables|Default|SetUpwardVelocity (Math|Interpolation|VInterpTo (Variables|Default|GetUpwardVelocity) "0, 0, 0" (Utilities|Time|GetWorldDeltaSeconds) 2e+01)))))
    (:then_1
      (if (and true (> _returnvalue_2 1.2e+03))
        (Variables|Default|SetForwardVelocity (/ (Variables|Default|GetForwardVelocity) _returnvalue_3))
        (Variables|Default|SetUpwardVelocity (/ (Variables|Default|GetUpwardVelocity) _returnvalue_3))
        (Variables|Default|SetThrust 3.0)
        (Development|PrintString "out of bounds")))
    (:then_2
      (Physics|SetPhysicsLinearVelocity (Variables|Default|GetSpaceship) (+ (Variables|Default|GetForwardVelocity) (Variables|Default|GetUpwardVelocity)) false "None"))))

(event Collision|EventHit
  (params (MyComp :type Primitive%20Component%20Object%20Reference) (Other :type Actor%20Object%20Reference) (OtherComp :type Primitive%20Component%20Object%20Reference) (bSelfMoved :type Boolean) (HitLocation :type Vector :default "0, 0, 0") (HitNormal :type Vector :default "0, 0, 0") (NormalImpulse :type Vector :default "0, 0, 0") (Hit :type Hit%20Result%20Structure%20%28by%20ref%29))
  (Development|PrintString "Hello"))

(event Input|ActionEvents|InputActionSupersonic
  (params (Key :type Key%20Structure :default "None"))
  (:Pressed
    (bind _output_get (Variables|Default|SetSupersonicSpeed true)))
  (:Released
    (Variables|Default|SetSupersonicSpeed false)))

(event Input|AxisEvents|InputAxisThrust
  (params (AxisValue :type Float%20%28single-precision%29))
  (Utilities|FlowControl|Sequence
    (:then_0
      (if (stale Input|ActionEvents|InputActionSupersonic _output_get)
        (if (not (Math|Float|NearlyEqual(Float) AxisValue 0.0 0.1))
          (Variables|Default|SetThrust (Math|Interpolation|FInterpTo (Variables|Default|GetThrust) (Math|Float|Lerp 0.0 (Variables|Default|GetMaxThrust) (/ (+ AxisValue 1.0) 0.1)) (Utilities|Time|GetWorldDeltaSeconds) 1.0)))
        (elif (not (not (Math|Float|NearlyEqual(Float) AxisValue 0.0 0.1)))
          (Variables|Default|SetThrust (Math|Interpolation|FInterpTo (Variables|Default|GetThrust) (Math|Float|Lerp 0.0 (Variables|Default|GetMaxThrust) (/ (+ AxisValue 1.0) 2.0)) (Utilities|Time|GetWorldDeltaSeconds) 0.2)))))
    (:then_1
      (Variables|Default|SetForwardVelocity (* (Math|Vector|GetForwardVector (Variables|Default|GetSpaceship)) (Variables|Default|GetThrust))))))

(event Input|AxisEvents|InputAxisMoveUp
  (params (AxisValue :type Float%20%28single-precision%29))
  (Class|PrimitiveComponent|AddTorqueinDegrees (Variables|Default|GetSpaceship) (* (Math|Vector|GetRightVector (Variables|Default|GetSpaceship)) (* AxisValue (Variables|Default|GetForwardTorquePower))) "None" true))

(event Input|AxisEvents|InputAxisMoveRight
  (params (AxisValue :type Float%20%28single-precision%29))
  (Class|PrimitiveComponent|AddTorqueinDegrees (Variables|Default|GetSpaceship) (* (Math|Vector|GetUpVector (Variables|Default|GetSpaceship)) (* AxisValue (Variables|Default|GetForwardTorquePower))) "None" true))

(event Input|AxisEvents|InputAxisRoll
  (params (AxisValue :type Float%20%28single-precision%29))
  (Class|PrimitiveComponent|AddTorqueinDegrees (Variables|Default|GetSpaceship) (* (Math|Vector|GetForwardVector (Variables|Default|GetSpaceship)) (* AxisValue (Variables|Default|GetForwardTorquePower))) "None" true))

(fn ConstructionScript)