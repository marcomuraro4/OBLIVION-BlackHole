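; BP_BlackHole is a black hole actor whose material is driven live by OSC messages.
; On BeginPlay it creates a dynamic instance of M_BlackHole_Inst on its static mesh and starts an OSC server listening on localhost.
; Each received message's address, minus its first character, becomes the scalar parameter name, and its first float becomes the value.
; Address and value are also printed on screen for debugging.
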(event Custom|Message%20Received
  (params (Message :type OSC%20Message%20Structure%20%28by%20ref%29) (IPAddress :type String) (Port :type Integer))
  (Utilities|FlowControl|Sequence
    (:then_0
      (bind _returnvalue (Class|OSCManager|GetOSCMessageAddress Message))
      (bind _returnvalue_2 (Class|OSCManager|GetOSCAddressFullPath _returnvalue))
      (Development|PrintString _returnvalue_2 true true "(R=0.000000,G=0.660000,B=1.000000,A=1.000000)" 5.0))
    (:then_1
      (bind _value (Class|OSCManager|GetFloat Message))
      (Development|PrintString (Utilities|String|ToString(Float) _value) true true "(R=0.000000,G=0.660000,B=1.000000,A=1.000000)" 5.0))
    (:then_2
      (Rendering|Material|SetScalarParameterValue (Variables|Default|GetBlackHoleDynamicInstance) (Utilities|String|StringToName (Utilities|String|GetSubstring _returnvalue_2 1 200)) _value :!class /Script/Engine.MaterialInstanceDynamic))))

(event EventBeginPlay
  (Utilities|FlowControl|Sequence
    (:then_0
      (bind _returnvalue (Rendering|Material|CreateDynamicMaterialInstance (Variables|Default|GetStaticMesh) 0 "/Game/MySpaceScene/M_BlackHole_Inst.M_BlackHole_Inst" "None" :!class /Script/Engine.PrimitiveComponent))
      (Variables|Default|SetBlackHoleDynamicInstance _returnvalue))
    (:then_1
      (bind _returnvalue_2 (Class|OSCManager|CreateOSCServer "127.0.0.1" 57121 false true "OSCServer" 0))
      (bind _output_get (Variables|Default|SetOscServer _returnvalue_2))
      (EventDispatchers|BindEventtoOnOscMessageReceived _output_get (delegate Custom|Message%20Received)))))

(event Collision|EventActorBeginOverlap
  (params (OtherActor :type Actor%20Object%20Reference)))

(event EventTick
  (params (DeltaSeconds :type Float%20%28single-precision%29)))

(fn ConstructionScript)